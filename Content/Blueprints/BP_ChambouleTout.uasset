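; Carnival can-knockdown (chamboule-tout) attraction that takes over when the third-person character overlaps it.
; On overlap it locks the player, blends to its camera, shows a crosshair cursor, passes the ball spawn transform and creates a force widget; LeaveGame restores control.
; EndGame waits briefly, shows a win or lose widget based on whether BP_Cans' list is empty, then resets by destroying balls and respawning the cans.
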(event Custom|EndGame
  (Utilities|FlowControl|Delay 1.5)
  (if (not (Variables|Default|GetResult))
    (CallFunction|MakeResult)
    (Utilities|FlowControl|Delay 4.0)
    (CallFunction|ResetGame)))

(event Collision|EventActorBeginOverlap
  (params (OtherActor :type Actor%20Object%20Reference))
  (bind _returnvalue (Game|GetPlayerController 0))
  (bind _asbp_third_person_character (Utilities|Casting|CastToBP_ThirdPersonCharacter OtherActor))
  (Variables|/Game/ThirdPerson/Blueprints/BP_ThirdPersonCharacter.BP_ThirdPersonCharacter_C|SetActualAttraction _asbp_third_person_character self)
  (Default|LockPlayer _asbp_third_person_character false)
  (Game|Player|SetViewTargetwithBlend _returnvalue (Components|GetOwner (Variables|Composants|GetCamera)) 1.0 "VTBlend_Linear" 0.0 false)
  (Variables|/Script/Engine.PlayerController|SetCurrentMouseCursor _returnvalue "Crosshairs")
  (Variables|/Script/Engine.PlayerController|SetbShowMouseCursor _returnvalue true)
  (bind _asbp_third_person_character_2 (Utilities|Casting|CastToBP_ThirdPersonCharacter (Game|GetPlayerCharacter 0)))
  (Variables|/Game/ThirdPerson/Blueprints/BP_ThirdPersonCharacter.BP_ThirdPersonCharacter_C|SetChamboulleToutActif _asbp_third_person_character_2 true)
  (Variables|/Game/ThirdPerson/Blueprints/BP_ThirdPersonCharacter.BP_ThirdPersonCharacter_C|SetBallSpawn _asbp_third_person_character_2 (Transformation|GetWorldTransform (Variables|Composants|GetStaticMesh)))
  (bind _returnvalue_2 (UserInterface|CreateWidget "/Game/Blueprints/WB_BallForce.WB_BallForce_C" (Game|GetPlayerController 0)))
  (Variables|Default|SetWB_BallForce _returnvalue_2))

(fn ConstructionScript)

(fn ResetGame
  (bind _asbp_third_person_character (Utilities|Casting|CastToBP_ThirdPersonCharacter (Game|GetPlayerCharacter 0)))
  (Default|DestroyAllBall _asbp_third_person_character)
  (bind _returnvalue (Actor|GetActorOfClass "/Game/Blueprints/BP_Cans.BP_Cans_C"))
  (Game|SpawnActorfromClass "/Game/Blueprints/BP_Cans.BP_Cans_C" (Transformation|GetActorTransform _returnvalue) "Undefined" "MultiplyWithRoot" 0 0)
  (Widget|RemovefromParent (Variables|Default|GetResultWidget))
  (Variables|Default|SetResult false)
  (Actor|DestroyActor _returnvalue))

(fn Win
  (bind _returnvalue (UserInterface|CreateWidget "/Game/Blueprints/WB_Win.WB_Win_C" (Game|GetPlayerController 0)))
  (UserInterface|Viewport|AddtoViewport _returnvalue 0)
  (Variables|Default|SetResultWidget _returnvalue))

(fn Loose
  (bind _returnvalue (UserInterface|CreateWidget "/Game/Blueprints/WB_Loose.WB_Loose_C" (Game|GetPlayerController 0)))
  (UserInterface|Viewport|AddtoViewport _returnvalue 0)
  (Variables|Default|SetResultWidget _returnvalue))

(fn MakeResult
  (Variables|Default|SetResult true)
  (bind _returnvalue (Actor|GetActorOfClass "/Game/Blueprints/BP_Cans.BP_Cans_C"))
  (if (== (Utilities|Array|Length (Variables|/Game/Blueprints/BP_Cans.BP_Cans_C|GetCanList _returnvalue)) 0)
    (bind _returnvalue_2 (Actor|GetActorOfClass "BP_ChambouleTout_C"))
    (CallFunction|Win _returnvalue_2)
    (else
      (bind _returnvalue_3 (Actor|GetActorOfClass "BP_ChambouleTout_C"))
      (CallFunction|Loose _returnvalue_3))))

(fn LeaveGame
  (params (BP%20Third%20Person%20Character :type BP%20Third%20Person%20Character%20Object%20Reference))
  (bind _returnvalue (Game|GetPlayerController 0))
  (Game|Player|SetViewTargetwithBlend _returnvalue BP%20Third%20Person%20Character 1.0 "VTBlend_Linear" 0.0 false)
  (Default|LockPlayer BP%20Third%20Person%20Character true)
  (Variables|/Script/Engine.PlayerController|SetbShowMouseCursor _returnvalue false)
  (Variables|/Game/ThirdPerson/Blueprints/BP_ThirdPersonCharacter.BP_ThirdPersonCharacter_C|SetChamboulleToutActif BP%20Third%20Person%20Character false))