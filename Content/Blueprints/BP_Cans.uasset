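; BP_Cans tracks a group of cans in a knock-down (chamboule-tout) game and resets the game once all have left it.
; One tick after BeginPlay, it moves its Box 30 units above the actor's origin and records the overlapping BP_Can actors.
; Each end overlap removes that can from the list, and an empty list calls ResetGame on the BP_ChambouleTout found in the level.
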(event Collision|EventActorEndOverlap
  (params (OtherActor :type Actor%20Object%20Reference))
  (bind _canlist (Variables|Default|GetCanList))
  (if (Utilities|Array|ContainsItem (Variables|Default|GetCanList) OtherActor)
    (Utilities|Array|RemoveItem _canlist OtherActor)
    (if (== (Utilities|Array|Length _canlist) 0)
      (bind _returnvalue (Actor|GetActorOfClass "/Game/Blueprints/BP_ChambouleTout.BP_ChambouleTout_C"))
      (Default|ResetGame _returnvalue))))

(event EventBeginPlay
  (Utilities|FlowControl|DelayUntilNextTick)
  (Transformation|SetWorldLocation (Variables|Default|GetBox) (+ (Transformation|GetActorLocation) "0.000000,0.000000,30.000000") false false)
  (Variables|Default|SetCanList (Collision|GetOverlappingActors "/Game/Blueprints/BP_Can.BP_Can_C" :!class /Script/Engine.Actor)))

(fn ConstructionScript)