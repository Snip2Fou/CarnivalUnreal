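; Game instance Blueprint that holds the player's Money balance and provides functions to spend, receive and check it.
; Pay subtracts a price without checking funds itself, while CheckMoney separately reports whether the balance covers a price.
; Pay and ReceiveMoney then find BP_ThirdPersonCharacter with GetActorOfClass and push the new balance to its GeneralUI through SetText.
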(fn Pay
  (params (Price :type Integer))
  (bind _output_get (Variables|Default|SetMoney (- (Variables|Default|GetMoney) Price)))
  (bind _returnvalue (Actor|GetActorOfClass "/Game/ThirdPerson/Blueprints/BP_ThirdPersonCharacter.BP_ThirdPersonCharacter_C"))
  (Default|SetText (Variables|/Game/ThirdPerson/Blueprints/BP_ThirdPersonCharacter.BP_ThirdPersonCharacter_C|GetGeneralUI _returnvalue) _output_get))

(fn ReceiveMoney
  (params (Money :type Integer))
  (bind _output_get (Variables|Default|SetMoney (+ (Variables|Default|GetMoney) Money)))
  (bind _returnvalue (Actor|GetActorOfClass "/Game/ThirdPerson/Blueprints/BP_ThirdPersonCharacter.BP_ThirdPersonCharacter_C"))
  (Default|SetText (Variables|/Game/ThirdPerson/Blueprints/BP_ThirdPersonCharacter.BP_ThirdPersonCharacter_C|GetGeneralUI _returnvalue) _output_get))

(fn CheckMoney
  (params (Price :type Integer))
  (return (>= (Variables|Default|GetMoney) Price)))