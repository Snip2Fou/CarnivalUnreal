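; BP_Cans manages the group of cans in the Chamboule-Tout (can knockdown) game.
; One second after BeginPlay it moves its Box just above the actor and gathers overlapping BP_Can actors into a master list and an alive list.
; Cans leaving the Box drop from the alive list, and the last one out calls EndGame on BP_ChambouleTout.
; ResetCans resets every can and restores the alive list.
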(event OnComponentEndOverlap(Box)
  (params (OverlappedComponent :type Primitive%20Component%20Object%20Reference) (OtherActor :type Actor%20Object%20Reference) (OtherComp :type Primitive%20Component%20Object%20Reference) (OtherBodyIndex :type Integer))
  (bind _alivecanlist (Variables|Default|GetAliveCanList))
  (bind _asbp_can (Utilities|Casting|CastToBP_Can OtherActor))
  (if (Utilities|Array|ContainsItem (Variables|Default|GetAliveCanList) _asbp_can)
    (Utilities|Array|RemoveItem _alivecanlist _asbp_can)
    (if (== (Utilities|Array|Length _alivecanlist) 0)
      (bind _returnvalue (Actor|GetActorOfClass "/Game/Blueprints/ChambouleTout/BP_ChambouleTout.BP_ChambouleTout_C"))
      (Default|EndGame _returnvalue))))

(event EventBeginPlay
  (bind _canlist (Variables|Default|GetCanList))
  (Utilities|FlowControl|Delay 1.0)
  (Transformation|SetWorldLocation (Variables|Default|GetBox) (+ (Transformation|GetActorLocation) "0.000000,0.000000,30.000000") false false)
  (for _array_element (Collision|GetOverlappingActors "/Game/Blueprints/ChambouleTout/BP_Can.BP_Can_C" :!class /Script/Engine.Actor)
    (bind _asbp_can (Utilities|Casting|CastToBP_Can _array_element)
      (:then
        (Utilities|Array|Add _canlist _asbp_can))
      (:CastFailed
        (Development|PrintText "Hello"))))
  (Variables|Default|SetAliveCanList _canlist))

(fn ConstructionScript)

(fn ResetCans
  (Development|PrintText "Rest Cans")
  (for _array_element (Variables|Default|GetCanList)
    (Default|ResetCan _array_element))
  (Variables|Default|SetAliveCanList (Variables|Default|GetCanList)))