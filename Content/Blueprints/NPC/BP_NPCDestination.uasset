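; BP_NPCDestination is an NPC destination actor that doubles as a spawner for BP_NPC when its Type is set to one particular enum value.
; On BeginPlay, that type starts a looping one-second timer that calls SpawnNPC at the actor's transform.
; SpawnNPC stops once its counter reaches 25, and the counter rises on every attempt, even if collision prevents the spawn.
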(event EventBeginPlay
  (if (Utilities|Enum|Equal(Enum) (Variables|Default|GetType) "NewEnumerator1")
    (Utilities|Time|SetTimerbyFunctionName 0 "SpawnNPC" 1.0 true)))

(fn ConstructionScript)

(fn SpawnNPC
  (if (< (Variables|Default|GetNbNPC) 25)
    (Game|SpawnActorfromClass "/Game/Blueprints/NPC/BP_NPC.BP_NPC_C" (Transformation|GetActorTransform) "AdjustIfPossibleButDontSpawnIfColliding" "MultiplyWithRoot" 0 0)
    (Variables|Default|SetNbNPC (+ (Variables|Default|GetNbNPC) 1))))