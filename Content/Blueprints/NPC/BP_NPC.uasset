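; BP_NPC is a wandering AI character that roams between BP_NPCDestination actors placed in the level.
; On BeginPlay it caches all destinations, then loops AI moves to random reachable points around a randomly picked one, retrying on failure.
; After a successful move it destroys itself if another random pick, not necessarily the destination just reached, has a specific type; otherwise it moves again.
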(event Custom|AIMove
  (bind _npc_destination (Variables|Default|GetNPC%20Destination))
  (bind _outitem (Utilities|Array|Random _npc_destination))
  (AI|AIMoveTo self (.RandomLocation (AI|Navigation|GetRandomReachablePointinRadius (Transformation|GetActorLocation _outitem) 1e+03 0 0)) 0 5.0 false
    (:OnSuccess
      (if (Utilities|Enum|Equal(Enum) (Variables|/Game/Blueprints/NPC/BP_NPCDestination.BP_NPCDestination_C|GetType _outitem) "NewEnumerator2")
        (Actor|DestroyActor)
        (else
          (CallFunction|AIMove :!label _label))))
    (:OnFail
      (goto _label))))

(event EventBeginPlay
  (bind _outactors (Actor|GetAllActorsOfClass "/Game/Blueprints/NPC/BP_NPCDestination.BP_NPCDestination_C"))
  (Variables|Default|SetNPC%20Destination _outactors)
  (CallFunction|AIMove))

(fn ConstructionScript)