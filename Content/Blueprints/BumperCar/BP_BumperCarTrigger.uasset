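; Bumper car attraction trigger that puts the player into a randomly chosen car for a timed ride.
; Entering the box blends the camera, swaps possession and input context, and starts a countdown UI.
; Timeout or the player's car leaving the arena box returns view to the character, with OutCar restoring possession and resetting cars.
; A looping timer randomly recolors spotlights, and any car leaving the arena gets TPOutCar called.
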(event OnComponentBeginOverlap(PlayerTriggerBox)
  (params (OverlappedComponent :type Primitive%20Component%20Object%20Reference) (OtherActor :type Actor%20Object%20Reference) (OtherComp :type Primitive%20Component%20Object%20Reference) (OtherBodyIndex :type Integer) (bFromSweep :type Boolean) (SweepResult :type Hit%20Result%20Structure%20%28by%20ref%29))
  (bind _returnvalue (Game|GetPlayerController 0))
  (bind _playerbumpercar (Variables|Default|GetPlayerBumperCar))
  (bind _asbp_third_person_character (Utilities|Casting|CastToBP_ThirdPersonCharacter OtherActor))
  (Default|LockPlayer _asbp_third_person_character false)
  (Variables|/Game/ThirdPerson/Blueprints/BP_ThirdPersonCharacter.BP_ThirdPersonCharacter_C|SetActualAttraction _asbp_third_person_character self)
  (Game|Player|SetViewTargetwithBlend _returnvalue _playerbumpercar 1.0 "VTBlend_Linear" 0.0 false)
  (Utilities|FlowControl|Delay 1.0)
  (Input|AddMappingContext (PlayerController|LocalPlayerSubsystems|GetEnhancedInputLocalPlayerSubsystem _returnvalue) "/Game/ThirdPerson/Input/IMC_BumperCar.IMC_BumperCar" 0 "(bIgnoreAllPressedKeysUntilRelease=True,bForceImmediately=False,bNotifyUserSettings=False)")
  (Pawn|Possess _returnvalue _playerbumpercar)
  (CallFunction|SpawnUI)
  (bind _returnvalue_2 (Utilities|Time|SetTimerbyEvent (delegate Custom|CustomEvent_0) 1.0 true))
  (Variables|Default|SetGameTimerHandle _returnvalue_2))

(event OnComponentEndOverlap(CarOutBox)
  (params (OverlappedComponent :type Primitive%20Component%20Object%20Reference) (OtherActor :type Actor%20Object%20Reference) (OtherComp :type Primitive%20Component%20Object%20Reference) (OtherBodyIndex :type Integer))
  (bind _asbp_bumper_car_vechicles (Utilities|Casting|CastToBP_BumperCarVechicles OtherActor))
  (Default|TPOutCar _asbp_bumper_car_vechicles)
  (if (== _asbp_bumper_car_vechicles (Variables|Default|GetPlayerBumperCar))
    (bind _returnvalue (Actor|GetActorOfClass "/Game/ThirdPerson/Blueprints/BP_ThirdPersonCharacter.BP_ThirdPersonCharacter_C"))
    (CallFunction|LeaveGame _returnvalue)
    (Utilities|Time|ClearandInvalidateTimerbyHandle (Variables|Default|GetGameTimerHandle))))

(event Custom|CustomEvent
  (for _array_element (Variables|Default|GetLightList)
    (Rendering|Components|Light|SetLightColor _array_element (Math|Conversions|ToLinearColor(Color) (.OutItem (Utilities|Array|Random (Variables|Default|GetLightColors)))) true)))

(event Custom|CustomEvent_0
  (bind _output_get (Variables|Default|SetGameTimer (- (Variables|Default|GetGameTimer) 1)))
  (Default|SetText (Variables|Default|GetGeneralUI) (Utilities|Text|ToText(String) (Utilities|String|Append (Utilities|String|ToString(Integer) (/ _output_get 60)) ":" (Utilities|String|ToString(Integer) (Class|KismetMathLibrary|PercentInt64Int64 _output_get 60)))))
  (if (== (Variables|Default|GetGameTimer) 0)
    (bind _returnvalue (Actor|GetActorOfClass "/Game/ThirdPerson/Blueprints/BP_ThirdPersonCharacter.BP_ThirdPersonCharacter_C"))
    (CallFunction|LeaveGame _returnvalue)
    (Utilities|Time|ClearandInvalidateTimerbyHandle (Variables|Default|GetGameTimerHandle))))

(event EventBeginPlay
  (bind _lightlist (Variables|Default|GetLightList))
  (bind _caroutbox (Variables|Default|GetCarOutBox))
  (bind _outactors (Actor|GetAllActorsOfClass "/Game/Blueprints/BumperCar/BP_BumperCarVechicles.BP_BumperCarVechicles_C"))
  (Variables|Default|SetBumperCars _outactors)
  (Variables|Default|SetPlayerBumperCar (.OutItem (Utilities|Array|Random _outactors)))
  (Utilities|Array|Add _lightlist (Variables|Default|GetSpotLight3))
  (Utilities|Array|Add _lightlist (Variables|Default|GetSpotLight2))
  (Utilities|Array|Add _lightlist (Variables|Default|GetSpotLight1))
  (Utilities|Array|Add _lightlist (Variables|Default|GetSpotLight))
  (Utilities|Time|SetTimerbyEvent (delegate Custom|CustomEvent) 0.2 true)
  (Utilities|FlowControl|DelayUntilNextTick)
  (Transformation|SetWorldLocation _caroutbox (+ (Transformation|GetWorldLocation _caroutbox) "0.000000,0.000000,500.000000") false false))

(fn ConstructionScript)

(fn LeaveGame
  (params (BP%20Third%20Person%20Character :type BP%20Third%20Person%20Character%20Object%20Reference))
  (Widget|RemovefromParent (Variables|Default|GetGeneralUI))
  (Game|Player|SetViewTargetwithBlend (Game|GetPlayerController 0) BP%20Third%20Person%20Character 1.0 "VTBlend_Linear" 0.0 false)
  (Default|LockPlayer BP%20Third%20Person%20Character true)
  (Utilities|Time|SetTimerbyEvent (EventDispatchers|CreateEvent :!event OutCar) 1.0))

(fn OutCar
  (bind _returnvalue (Game|GetPlayerController 0))
  (Input|RemoveMappingContext (PlayerController|LocalPlayerSubsystems|GetEnhancedInputLocalPlayerSubsystem _returnvalue) "/Game/ThirdPerson/Input/IMC_BumperCar.IMC_BumperCar" "(bIgnoreAllPressedKeysUntilRelease=True,bForceImmediately=False,bNotifyUserSettings=False)")
  (Pawn|UnPossess _returnvalue)
  (bind _returnvalue_2 (Actor|GetActorOfClass "/Game/ThirdPerson/Blueprints/BP_ThirdPersonCharacter.BP_ThirdPersonCharacter_C"))
  (Pawn|Possess _returnvalue _returnvalue_2)
  (for _array_element (Variables|Default|GetBumperCars)
    (Default|ResetCar _array_element)))

(fn SpawnUI
  (bind _returnvalue (UserInterface|CreateWidget "/Game/Blueprints/BumperCar/WB_BumperCarUI.WB_BumperCarUI_C"))
  (Variables|Default|SetGeneralUI _returnvalue)
  (UserInterface|Viewport|AddtoViewport _returnvalue 0))