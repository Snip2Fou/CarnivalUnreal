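; Drivable bumper car for an attraction, controlled through Enhanced Input.
; Move input applies planar force along the mesh's forward vector, while turn input directly yaws the mesh.
; The leave input finds the third-person character and calls LeaveGame on its current attraction.
; ResetCar returns the car to its BeginPlay transform with physics re-enabled; TPOutCar disables physics and parks it below that spot.
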(event Input|EnhancedActionEvents|EnhancedInputActionIA_LeaveAttraction
  (params (ActionValue :type Boolean) (ElapsedSeconds :type Float%20%28double-precision%29) (TriggeredSeconds :type Float%20%28double-precision%29) (InputAction :type Input%20Action%20Object%20Reference :default "/Game/ThirdPerson/Input/Actions/IA_LeaveAttraction.IA_LeaveAttraction"))
  (:Started
    (bind _returnvalue (Actor|GetActorOfClass "/Game/ThirdPerson/Blueprints/BP_ThirdPersonCharacter.BP_ThirdPersonCharacter_C"))
    (Default|LeaveGame (Variables|/Game/ThirdPerson/Blueprints/BP_ThirdPersonCharacter.BP_ThirdPersonCharacter_C|GetActualAttraction _returnvalue) _returnvalue)))

(event Input|EnhancedActionEvents|EnhancedInputActionIA_BumperMove
  (params (ActionValue :type Float%20%28double-precision%29) (ElapsedSeconds :type Float%20%28double-precision%29) (TriggeredSeconds :type Float%20%28double-precision%29) (InputAction :type Input%20Action%20Object%20Reference :default "/Game/ThirdPerson/Input/Actions/IA_BumperMove.IA_BumperMove"))
  (bind _staticmesh (Variables|Default|GetStaticMesh))
  (Physics|AddForce _staticmesh (* (* (Math|Vector|GetForwardVector _staticmesh) ActionValue) "10000.000000,10000.000000,0.000000") "None" false))

(event Input|EnhancedActionEvents|EnhancedInputActionIA_BumperTurn
  (params (ActionValue :type Float%20%28double-precision%29) (ElapsedSeconds :type Float%20%28double-precision%29) (TriggeredSeconds :type Float%20%28double-precision%29) (InputAction :type Input%20Action%20Object%20Reference :default "/Game/ThirdPerson/Input/Actions/IA_BumperTurn.IA_BumperTurn"))
  (bind _staticmesh (Variables|Default|GetStaticMesh))
  (Transformation|SetWorldRotation _staticmesh (Math|Rotator|CombineRotators (Transformation|GetWorldRotation _staticmesh) (Math|Rotator|MakeRotator 0.0 0.0 (* ActionValue 1.0))) false false))

(event EventBeginPlay
  (Variables|Default|SetSpawnPoint (Transformation|GetActorTransform)))

(fn ConstructionScript)

(fn ResetCar
  (Physics|SetSimulatePhysics (Variables|Default|GetStaticMesh) false)
  (Transformation|SetActorTransform (Variables|Default|GetSpawnPoint))
  (Physics|SetSimulatePhysics (Variables|Default|GetStaticMesh) true))

(fn TPOutCar
  (Physics|SetSimulatePhysics (Variables|Default|GetStaticMesh) false)
  (Transformation|SetActorLocation (+ (.Location (Math|Transform|BreakTransform (Variables|Default|GetSpawnPoint))) "0.000000,0.000000,-500.000000") false false))